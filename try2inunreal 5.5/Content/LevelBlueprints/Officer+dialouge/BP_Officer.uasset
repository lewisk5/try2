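; BP_Officer is an officer character that shows dialogue one line at a time.
; Each Talk event advances an index into the dialogue array and writes that line to a dialogue widget, created if none is valid.
; Every displayed line also adds a new control descriptions widget, which this graph never removes.
; Past the last line, it removes the dialogue widget and resets the index so the conversation can replay.
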(event EventBeginPlay)

(event Collision|EventActorBeginOverlap
  (params (OtherActor :type Actor%20Object%20Reference)))

(event EventTick
  (params (DeltaSeconds :type Float%20%28single-precision%29)))

(event EventTalk
  (Math|Integer|IncrementInt (Variables|Default|Gettalk%20index)
    (:%20%20
      (if (< (Variables|Default|Gettalk%20index) (Utilities|Array|Length (Variables|Default|Getdialouge)))
        (Variables|Default|GetUI
          (:then
            _)
          (:else
            (bind _returnvalue (UserInterface|CreateWidget "/Game/LevelBlueprints/Officer+dialouge/BP_dialougewidget.BP_dialougewidget_C" (Game|GetPlayerController 0)))
            (bind _output_get (Variables|Default|SetUI _returnvalue))
            (UserInterface|Viewport|AddtoViewport _output_get 0)))
        (Rendering|Components|TextRender|SetText (Variables|/Game/LevelBlueprints/Officer+dialouge/BP_dialougewidget.BP_dialougewidget_C|GetTextBlock_56 (Variables|Default|GetUI)) (Utilities|Text|ToText(String) (Utilities|Array|Get(acopy) (Variables|Default|Getdialouge) (Variables|Default|Gettalk%20index))))
        (bind _returnvalue_2 (UserInterface|CreateWidget "/Game/WidgetsandHUD/Controldescriptions.Controldescriptions_C"))
        (UserInterface|Viewport|AddtoViewport _returnvalue_2 0)
        (else
          (Widget|RemovefromParent (Variables|Default|GetUI))
          (Variables|Default|Settalk%20index -1)
          (Variables|Default|SetUI 0))))))

(fn ConstructionScript)